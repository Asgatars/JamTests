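; BP_MyController is a controller Blueprint that turns movement axis input into direct transform changes on the player pawn.
; MoveForward offsets the pawn locally along Direction without sweep, and MoveRight yaws it by TurnRate, both scaled by the delta time cached on Tick.
; A Drift function, not called in this file, offsets the player controller actor, rather than the pawn, along the BP_Ufo collision's forward vector.
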(event `self.ReceiveBeginPlay`)

(event `self.ReceiveTick`
  (params (DeltaSeconds :type "Float (single-precision)"))
  (set `self.DeltaSecond` DeltaSeconds))

(event `InputAxis|MoveForward`
  (params (AxisValue :type "Float (single-precision)"))
  (`self.K2_AddActorLocalOffset` (`GameplayStatics.GetPlayerPawn` 0) (* (* (`self.Direction`) AxisValue) (`self.DeltaSecond`)) false false))

(event `InputAxis|MoveRight`
  (params (AxisValue :type "Float (single-precision)"))
  (`self.K2_AddActorLocalRotation` (`GameplayStatics.GetPlayerPawn` 0) (`KismetMathLibrary.MakeRotator` 0.0 0.0 (* (* AxisValue (`self.TurnRate`)) (`self.DeltaSecond`))) false false))

(fn `Drift`
  (bind _asbp_ufo (cast `/Game/Blueprint/Caracter/BP_Ufo` (`GameplayStatics.GetPlayerPawn` 0)))
  (`self.K2_AddActorWorldOffset` (`GameplayStatics.GetPlayerController` 0) (* (* (`SceneComponent.GetForwardVector` (`/Game/Blueprint/Caracter/BP_Ufo.Collision` _asbp_ufo)) (`self.DeltaSecond`)) 1000.0) false false))

(fn `UserConstructionScript`)